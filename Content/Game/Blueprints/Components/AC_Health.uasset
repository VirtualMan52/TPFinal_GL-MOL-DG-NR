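; Actor component that tracks an actor's health, handling damage, healing and death.
; TakeDamage and Heal clamp CurrentHealth between zero and MaxHealth and broadcast OnHealthChanged with the requested signed change, ignoring calls while dead.
; Reaching zero through damage fires OnDeath and then sets IsDead.
; ResetHealth sets current and max values, broadcasts the update, and clears IsDead if health is positive.
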(event `ResetHealth`
  (params (`Current Health` :type Integer) (`Max Health` :type Integer))
  (set `self.CurrentHealth` `Current Health`)
  (set `self.MaxHealth` `Max Health`)
  (`self.OnHealthChanged` (`self.CurrentHealth`) (`self.MaxHealth`))
  (if (> (`self.CurrentHealth`) 0)
    (set `self.IsDead` false)))

(event `TakeDamage`
  (params (`Damage Amount` :type Integer))
  (if (not (`self.IsDead`))
    (bind _output_get (set `self.CurrentHealth` (`KismetMathLibrary.Clamp` (- (`self.CurrentHealth`) `Damage Amount`) 0 (`self.MaxHealth`))))
    (`self.OnHealthChanged` _output_get (`self.MaxHealth`) (* `Damage Amount` -1))
    (if (== (`self.CurrentHealth`) 0)
      (`self.OnDeath`)
      (set `self.IsDead` true))))

(event `Heal`
  (params (`Heal Amount` :type Integer))
  (if (not (`self.IsDead`))
    (bind _output_get (set `self.CurrentHealth` (`KismetMathLibrary.Clamp` (+ (`self.CurrentHealth`) `Heal Amount`) 0 (`self.MaxHealth`))))
    (`self.OnHealthChanged` _output_get (`self.MaxHealth`) `Heal Amount`)))
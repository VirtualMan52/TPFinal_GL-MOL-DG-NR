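; BP_MovingSaw is a saw blade trap that moves along local X while rotating and damages the player.
; On BeginPlay, the SawRoll timeline starts from an Offset time, driving blade position and compounding rotation onto its current transform, while saw audio plays from a random start point.
; Blade box overlap with player character 0 applies damage through AC_Health, then a brief Immunity delay blocks repeat hits.
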(event `self.ReceiveBeginPlay`
  ; Faire bouger la lame
  (`|ExecutionSequence`
    (:`then_0`
      (bind (_direction _rotation _location_x) (`Timeline|SawRoll` :`NewTime` (`self.Offset`) :!via `SetNewTime` :!label _label)
        (:`Update`
          (`SceneComponent.K2_SetRelativeTransform` (`self.saw_blade`) (`KismetMathLibrary.MakeTransform` (`KismetMathLibrary.MakeVector` _location_x) (`KismetMathLibrary.ComposeRotators` (`KismetMathLibrary.MakeRotator` 0.0 0.0 _rotation) (.rotation (`SceneComponent.GetRelativeTransform` (`self.saw_blade`)))) (.scale (`SceneComponent.GetRelativeTransform` (`self.saw_blade`)))) false false))))
    (:`then_1`
      (goto _label))
    (:`then_2`
      ; Jouer le son
      (`AudioComponent.Play` (`self.AudioSaw`) (`KismetMathLibrary.RandomFloatInRange` 0.0 7.0)))))

(event `self.Box_collider_Blade.OnComponentBeginOverlap`
  (params (OverlappedComponent :type "PrimitiveComponent Object Reference") (OtherActor :type "Actor Object Reference") (OtherComp :type "PrimitiveComponent Object Reference") (OtherBodyIndex :type Integer) (bFromSweep :type Boolean) (SweepResult :type "HitResult Structure (by ref)"))
  (bind _returnvalue (`GameplayStatics.GetPlayerCharacter` 0))
  ; Dammage
  (`/Engine/EditorBlueprintResources/StandardMacros.IsValid` OtherActor
    (:`Is Valid`
      (if (and (== OtherActor _returnvalue) (== (`self.Immunity`) false))
        (set `self.Immunity` true)
        (`/Game/Game/Blueprints/Components/AC_Health.TakeDamage` (`self.GetComponentByClass` _returnvalue "/Game/Game/Blueprints/Components/AC_Health.AC_Health_C") 10)
        (`KismetSystemLibrary.PrintString` "Saw damage")
        (`KismetSystemLibrary.Delay` 0.8)
        (set `self.Immunity` false)))))

(fn `UserConstructionScript`)
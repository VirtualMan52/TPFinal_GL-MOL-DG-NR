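; BP_EndDoor is a level exit door that sends the player to the level named in LevelName.
; When the third-person character overlaps its Trigger, it disables that character's input and calls TransitionTo on BP_GameInstance.
; It then saves the character stats of the player pawn, after the transition call.
; The door sound plays at the actor's location on BeginPlay, not on entry.
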(event `self.Trigger.OnComponentBeginOverlap`
  (params (OverlappedComponent :type "PrimitiveComponent Object Reference") (OtherActor :type "Actor Object Reference") (OtherComp :type "PrimitiveComponent Object Reference") (OtherBodyIndex :type Integer) (bFromSweep :type Boolean) (SweepResult :type "HitResult Structure (by ref)"))
  ; Transporte le joueur à un nouveau niveau lorsqu'il entre dans la porte
  (bind _asbp_third_person_character (cast `/Game/Game/Blueprints/Pawns_Characters/Player/BP_ThirdPersonCharacter` OtherActor))
  (`self.DisableInput` _asbp_third_person_character null)
  (bind _asbp_game_instance (cast `/Game/Game/Blueprints/BP_GameInstance` (`GameplayStatics.GetGameInstance`)))
  (`/Game/Game/Blueprints/BP_GameInstance.TransitionTo` _asbp_game_instance (`self.LevelName`))
  ; Sauvegarde les stats du personnage
  (bind _asbp_third_person_character_2 (cast `/Game/Game/Blueprints/Pawns_Characters/Player/BP_ThirdPersonCharacter` (`GameplayStatics.GetPlayerPawn` 0)))
  (`/Game/Game/Blueprints/Pawns_Characters/Player/BP_ThirdPersonCharacter.SaveCharacterStats` _asbp_third_person_character_2))

(event `self.ReceiveBeginPlay`
  ; Joue le son de la porte
  (`GameplayStatics.PlaySoundAtLocation` "/Game/Game/Audio/SFX/SoundWave/SW_EndDoor.SW_EndDoor" (`self.K2_GetActorLocation`) (struct) 1.0 1.0 0.0 "/Game/Game/Audio/SFX/Attenuation/SA_EndDoor.SA_EndDoor" null null null))

(fn `UserConstructionScript`)
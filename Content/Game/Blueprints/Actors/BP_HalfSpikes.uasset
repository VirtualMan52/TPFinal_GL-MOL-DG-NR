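; Rhythm-driven spike trap that fires on every other beat, odd or even depending on its Odd flag.
; On a matching Activate(Beat), it deals fixed damage through AC_Health to actors overlapping its HurtBox, then plays the spike sound.
; The Attack timeline then animates the Spikes' height, so damage lands once as the motion starts.
; The construction script applies an optional BaseMaterial to the base.
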(event `self.Activate`
  (params (Beat :type Integer))
  ; S'active seulement au beat pair/impair
  (if (== (mod Beat 2) (`KismetMathLibrary.SelectInt` 1 0 (`self.Odd`)))
    ; Endommage les acteurs dans la boîte de collision
    (for _array_element (`PrimitiveComponent.GetOverlappingActors` (`self.HurtBox`) null)
      (bind _returnvalue (`self.GetComponentByClass` _array_element "/Game/Game/Blueprints/Components/AC_Health.AC_Health_C"))
      (`/Engine/EditorBlueprintResources/StandardMacros.IsValid` _returnvalue
        (:`Is Valid`
          (`/Game/Game/Blueprints/Components/AC_Health.TakeDamage` _returnvalue 40))))
    ; Fais jouer le son
    (`GameplayStatics.PlaySoundAtLocation` "/Game/Game/Audio/SFX/SoundCue/SC_Spikes.SC_Spikes" (`self.K2_GetActorLocation`) (struct) 1.0 1.0 0.0 null null null null)
    ; Fais jouer l'animation des pics
    (bind (_direction _height) (`Timeline|Attack` :!via `PlayFromStart`)
      (:`Update`
        (`SceneComponent.K2_SetRelativeLocation` (`self.Spikes`) (`KismetMathLibrary.MakeVector` 0.0 0.0 _height) false false)))))

(fn `UserConstructionScript`
  ; Changement de matériel de la base si besoin
  (`/Engine/EditorBlueprintResources/StandardMacros.IsValid` (`self.BaseMaterial`)
    (:`Is Valid`
      (`PrimitiveComponent.SetMaterial` (`self.SpikeBase`) 0 (`self.BaseMaterial`)))))
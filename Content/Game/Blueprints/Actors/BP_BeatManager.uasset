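; BP_BeatManager is an actor that runs a musical beat, triggering beat-reactive objects in time with background music.
; It silences the Music audio at BeginPlay; Activate fades it in or out and starts or clears a looping half-second timer.
; Each tick advances a four-beat counter and sends it to BPI_BeatActivable actors in Activations, plus every BP_BeatTorch, gathered by class to avoid manual assignment.
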(event `self.ReceiveBeginPlay`
  ; Démarre la séquence musicale en arrière-plan
  (bind _output_get (set `self.Audio Component` (`AmbientSound.AudioComponent` (`self.Music`))))
  (`AudioComponent.FadeOut` _output_get 0.0 0.0 "Linear"))

(event `Beat`
  ; Compte chaque beat
  (set `self.BeatCounter` (+ (`self.BeatCounter`) 1))
  (if (> (`self.BeatCounter`) 4)
    (set `self.BeatCounter` (- (`self.BeatCounter`) 4)))
  (if (`self.Activated`)
    (`|ExecutionSequence`
      (:`then_0`
        ; Appelle tous les objets devant réagir au beat
        (for _array_element (`self.Activations`)
          (if (`KismetSystemLibrary.DoesImplementInterface` _array_element "/Game/Game/Blueprints/Interfaces/BPI_BeatActivable.BPI_BeatActivable_C")
            (message `/Game/Game/Blueprints/Interfaces/BPI_BeatActivable.Activate` _array_element (`self.BeatCounter`)))))
      (:`then_1`
        ; Appelle spécifiquement les torches (plus rapide que de les assigner manuellement)
        (bind _outactors (`GameplayStatics.GetAllActorsOfClass` "/Game/Game/Blueprints/Actors/BP_BeatTorch.BP_BeatTorch_C"))
        (for _array_element_2 _outactors
          (message `/Game/Game/Blueprints/Interfaces/BPI_BeatActivable.Activate` _array_element_2 (`self.BeatCounter`)))))))

(event `/Game/Game/Blueprints/Interfaces/BPI_Activable.Activate`
  (params (Active :type Boolean))
  (bind _audio_component (`self.Audio Component`))
  ; Permet de débuter/arrêter les activations musicales
  (bind _output_get (set `self.Activated` Active))
  (if _output_get
    (`AudioComponent.FadeIn` _audio_component 1.0 1.0 0.0 "Linear")
    (set `self.BeatCounter` 4)
    (bind _returnvalue (`KismetSystemLibrary.K2_SetTimerDelegate` (delegate `Beat`) 0.5 true))
    (set `self.Timer Handle` _returnvalue)
    (else
      (`AudioComponent.FadeOut` _audio_component 2.0 0.0 "Linear")
      (`KismetSystemLibrary.K2_ClearAndInvalidateTimerHandle` (`self.Timer Handle`)))))

(fn `UserConstructionScript`)
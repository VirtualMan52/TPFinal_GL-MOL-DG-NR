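; Interactable lever actor whose handle swings between two states, with an option to be usable only once.
; Interacted flips Pulled, calls ToggleLever, then disables further interaction through ToggleActivation when OneTime is set.
; ToggleLever prints Pulled and plays or reverses the LeverAnimation timeline, which drives the roll of ManchePivot.
; BeginPlay also calls ToggleLever after the parent's logic, so the handle animates according to its starting state.
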(event `self.ReceiveBeginPlay`
  (`parent.ReceiveBeginPlay`)
  (`self.ToggleLever`))

(event `ToggleLever`
  (`KismetSystemLibrary.PrintString` (`KismetStringLibrary.Conv_BoolToString` (`self.Pulled`)))
  (if (`self.Pulled`)
    (bind (_direction _newtrack_0) (`Timeline|LeverAnimation` :!label _label)
      (:`Update`
        (`SceneComponent.K2_SetRelativeRotation` (`self.ManchePivot`) (`KismetMathLibrary.MakeRotator` _newtrack_0) false false)))
    (else
      (goto _label :!via `Reverse`))))

(fn `Interacted`
  ; Change l'état du levier
  (set `self.Pulled` (not (`self.Pulled`)))
  (`self.ToggleLever`)
  ; Désactive l'interaction si le levier ne peut être qu'activé une fois
  (if (`self.OneTime`)
    (`self.ToggleActivation` false)))

(fn `UserConstructionScript`
  (`parent.UserConstructionScript`))
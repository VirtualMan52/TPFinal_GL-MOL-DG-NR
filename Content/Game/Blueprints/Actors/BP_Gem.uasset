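; BP_Gem is a collectible gem that hovers and spins until the player character touches it.
; A Timeline drives the mesh's height and yaw, restarting itself on finish to loop the animation.
; On overlap with BP_ThirdPersonCharacter, it registers its Key in BP_GameInstance through AddGem, spawns the NS_Collection effect at its location and destroys itself.
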(event `self.ReceiveBeginPlay`
  ; Fait jouer l'animation de rotation/hover du modèle de la gemme
  (bind (_direction _height _rotation) (`Timeline|Timeline` :!label _label)
    (:`Update`
      (`SceneComponent.K2_SetRelativeLocationAndRotation` (`self.StaticMesh`) (`KismetMathLibrary.MakeVector` 0.0 0.0 (* _height 15.0)) (`KismetMathLibrary.MakeRotator` 0.0 0.0 _rotation) false false))
    (:`Finished`
      (`self.Play Animation`))))

(event `Play Animation`
  ; Fait jouer l'animation de rotation/hover du modèle de la gemme
  (goto _label :!via `PlayFromStart`))

(event `self.StaticMesh.OnComponentBeginOverlap`
  (params (OverlappedComponent :type "PrimitiveComponent Object Reference") (OtherActor :type "Actor Object Reference") (OtherComp :type "PrimitiveComponent Object Reference") (OtherBodyIndex :type Integer) (bFromSweep :type Boolean) (SweepResult :type "HitResult Structure (by ref)"))
  ; Ajoute la gemme au GameInstance sur contact
  (cast `/Game/Game/Blueprints/Pawns_Characters/Player/BP_ThirdPersonCharacter` OtherActor)
  (bind _asbp_game_instance (cast `/Game/Blueprints/BP_GameInstance` (`GameplayStatics.GetGameInstance`)))
  (`/Game/Blueprints/BP_GameInstance.AddGem` _asbp_game_instance (`self.Key`))
  ; Effets visuels et disparition
  (`NiagaraFunctionLibrary.SpawnSystemAtLocation` "/Game/Game/VFX/Particle_System/NS_Collection.NS_Collection" (`self.K2_GetActorLocation`))
  (`self.K2_DestroyActor`))

(fn `UserConstructionScript`)
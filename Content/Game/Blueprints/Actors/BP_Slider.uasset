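; BP_Slider is a one-shot sliding actor that, per the author's comment, moves when the player presses E.
; Its Activate event runs once, plays the slider sound and saves the current location as the start point.
; A timeline then lerps the root component's location from that start to start plus the PositionDeFin offset, which is therefore relative to the starting position.
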(event `/Game/Game/Blueprints/Interfaces/BPI_Activable.Activate`
  (params (Active :type Boolean))
  (bind _returnvalue (`self.K2_GetActorLocation`))
  ; Quand le joueur appuie sur E, il fait bouger le BP_Slider. Mais seulement une fois. ( La position de départ est sauvegardé pour que la variable position de fin peut être additioné par dessus)
  (`/Engine/EditorBlueprintResources/StandardMacros.DoOnce` false
    (:`Completed`
      (`GameplayStatics.PlaySoundAtLocation` "/Game/Game/Audio/SFX/SoundWave/S_Slider.S_Slider" _returnvalue (struct) 3.0 1.0 1.0 "/Game/Game/Audio/SFX/Attenuation/SA_Slider.SA_Slider" null null null)
      (set `self.Position de départ` _returnvalue)
      (bind (_direction _valeur_float) (`Timeline|Timeline`)
        (:`Update`
          (`SceneComponent.K2_SetRelativeLocation` (`self.DefaultSceneRoot`) (`KismetMathLibrary.VLerp` (`self.Position de départ`) (+ (`self.Position de départ`) (`self.Position de fin`)) _valeur_float) false false))))))

(fn `UserConstructionScript`)
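; BP_SpikeBed is a beat-driven spike trap that strikes on the fourth beat.
; Its Activate event deals fixed damage through the AC_Health component of each actor overlapping HurtBox when the beat matches.
; It then plays a spike sound at its location and runs the Attack timeline, which drives the relative height of the Spikes component.
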(event `/Game/Game/Blueprints/Interfaces/BPI_BeatActivable.Activate`
  (params (Beat :type Integer))
  ; S'active seulement au quatrième beat
  (if (== Beat 4)
    ; Endommage les acteurs dans la boîte de collision
    (for _array_element (`PrimitiveComponent.GetOverlappingActors` (`self.HurtBox`) null)
      (bind _returnvalue (`self.GetComponentByClass` _array_element "/Game/Game/Blueprints/Components/AC_Health.AC_Health_C"))
      (`/Engine/EditorBlueprintResources/StandardMacros.IsValid` _returnvalue
        (:`Is Valid`
          (`/Game/Game/Blueprints/Components/AC_Health.TakeDamage` _returnvalue 40))))
    ; Fais jouer le son des spikes
    (`GameplayStatics.PlaySoundAtLocation` "/Game/Game/Audio/SFX/SoundCue/SC_Spikes.SC_Spikes" (`self.K2_GetActorLocation`) (struct) 1.0 1.0 0.0 null null null null)
    ; Fais jouer l'animation des spikes
    (bind (_direction _height) (`Timeline|Attack` :!via `PlayFromStart`)
      (:`Update`
        (`SceneComponent.K2_SetRelativeLocation` (`self.Spikes`) (`KismetMathLibrary.MakeVector` 0.0 0.0 _height) false false)))))

(fn `UserConstructionScript`)
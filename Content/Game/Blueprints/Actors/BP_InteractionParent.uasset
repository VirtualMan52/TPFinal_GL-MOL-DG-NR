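; BP_InteractionParent is a base actor for interactable objects that the player can approach and use.
; Its construction script places and sizes a trigger sphere from offset and range variables, and BeginPlay puts the interaction label on a widget component.
; The trigger registers and unregisters the actor with BP_ThirdPersonCharacter on overlap.
; ToggleUI shows or hides the prompt, and Interacted holds placeholder behaviour that only prints a message.
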(event `self.ReceiveBeginPlay`
  (bind _aswbp_interaction_ui (cast `/Game/Game/UI/WBP_InteractionUI` (`WidgetComponent.GetWidget` (`self.UI`))))
  (`/Game/Game/UI/WBP_InteractionUI.SetText` _aswbp_interaction_ui (`self.InteractionLabel`)))

(event `self.InteractionTrigger.OnComponentBeginOverlap`
  (params (OverlappedComponent :type "PrimitiveComponent Object Reference") (OtherActor :type "Actor Object Reference") (OtherComp :type "PrimitiveComponent Object Reference") (OtherBodyIndex :type Integer) (bFromSweep :type Boolean) (SweepResult :type "HitResult Structure (by ref)"))
  (bind _asbp_third_person_character (cast `/Game/Game/Blueprints/Pawns_Characters/Player/BP_ThirdPersonCharacter` OtherActor))
  (`/Game/Game/Blueprints/Pawns_Characters/Player/BP_ThirdPersonCharacter.AddInteraction` _asbp_third_person_character self))

(event `self.InteractionTrigger.OnComponentEndOverlap`
  (params (OverlappedComponent :type "PrimitiveComponent Object Reference") (OtherActor :type "Actor Object Reference") (OtherComp :type "PrimitiveComponent Object Reference") (OtherBodyIndex :type Integer))
  (bind _asbp_third_person_character (cast `/Game/Game/Blueprints/Pawns_Characters/Player/BP_ThirdPersonCharacter` OtherActor))
  (`/Game/Game/Blueprints/Pawns_Characters/Player/BP_ThirdPersonCharacter.RemoveInteraction` _asbp_third_person_character self))

(fn `Interacted`
  (`KismetSystemLibrary.PrintString` "Default interaction behaviour!"))

(fn `ToggleUI`
  (params (Visible :type Boolean))
  (`SceneComponent.SetVisibility` (`self.UI`) Visible false))

(fn `UserConstructionScript`
  (`SceneComponent.K2_SetRelativeTransform` (`self.InteractionTrigger`) (`self.InteractionOffset`) false false)
  (`SphereComponent.SetSphereRadius` (`self.InteractionTrigger`) (`self.InteractionRange`) true))
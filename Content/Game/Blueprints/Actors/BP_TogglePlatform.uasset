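; Rhythm platform actor that toggles between solid and gone on every N-th beat passed to its Activate event, set by Beats.
; UpdatePlatform applies the Active state on BeginPlay and after each toggle, switching the cube's collision immediately.
; Separate timelines scale the actor up or down, and it is hidden only once shrinking finishes.
; The construction script applies an optional material override to the cube.
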(event `self.ReceiveBeginPlay`
  ; Démarre la plateforme au bon état
  (`self.UpdatePlatform`))

(event `/Game/Game/Blueprints/Interfaces/BPI_BeatActivable.Activate`
  (params (Beat :type Integer))
  ; Change l'état de la plateforme à chaque certain beat
  (if (== (mod Beat (`self.Beats`)) 0)
    (set `self.Active` (not (`self.Active`)))
    (`self.UpdatePlatform`)))

(event `UpdatePlatform`
  ; Active/Désactive les collisions
  (if (`self.Active`)
    (`PrimitiveComponent.SetCollisionEnabled` (`self.Cube`) "QueryAndPhysics")
    (`self.SetActorHiddenInGame` false)
    ; Fais jouer l'animation sur la taille de la plateforme
    (bind (_direction _scale) (`Timeline|Scale_Up` :!via `PlayFromStart`)
      (:`Update`
        (`self.SetActorScale3D` (`KismetMathLibrary.MakeVector` _scale _scale _scale)))
      (:`Finished`
        ; Cache la plateforme si elle a été rapetissée
        (if (not (`self.Active`)) :!label _label
          (`self.SetActorHiddenInGame` true))))
    (else
      (`PrimitiveComponent.SetCollisionEnabled` (`self.Cube`) "NoCollision")
      (bind (_direction_2 _scale_2) (`Timeline|Scale_Down` :!via `PlayFromStart`)
        (:`Update`
          (`self.SetActorScale3D` (`KismetMathLibrary.MakeVector` _scale_2 _scale_2 _scale_2)))
        (:`Finished`
          (goto _label))))))

(fn `UserConstructionScript`
  (bind _material (`self.Material`))
  ; Change le matériau si besoin
  (`/Engine/EditorBlueprintResources/StandardMacros.IsValid` _material
    (:`Is Valid`
      (`PrimitiveComponent.SetMaterial` (`self.Cube`) 0 _material))))
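; BP_Plateforme is a platform that moves on its own once play begins.
; BeginPlay saves its starting location, plays a chain sound there and starts a timeline.
; Each timeline update lerps the root's relative location from that start to the start plus the PositionDeFin offset, without sweeping.
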(event `self.ReceiveBeginPlay`
  (bind _returnvalue (`self.K2_GetActorLocation`))
  ; Le BP_Plateforme bouge tout seul grâce au timeline, ( La position de départ est sauvegardé pour que la variable position de fin peut être additioné par dessus)
  (set `self.PositionDepart` _returnvalue)
  (`GameplayStatics.PlaySoundAtLocation` "/Game/sandbox/Marco/Sons/S_Chaines.S_Chaines" _returnvalue (struct) 5.0 2.0 0.0 "/Game/sandbox/Marco/Sons/SA_Chaines.SA_Chaines" null null null)
  (bind (_direction _float_valeur) (`Timeline|Timeline de la plateforme`)
    (:`Update`
      (`SceneComponent.K2_SetRelativeLocation` (`self.DefaultSceneRoot`) (`KismetMathLibrary.VLerp` (`self.PositionDepart`) (+ (`self.PositionDepart`) (`self.Position de fin`)) _float_valeur) false false))))

(fn `UserConstructionScript`)